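; Player controller component that drives a fade-in/fade-out scene scan post-process effect, toggled by StartScan and EndScan.
; A state machine advances normalized scan time on Tick, writing it and the pawn location to a material parameter collection and disabling Tick when faded out.
; Curves map time to camera FOV and blend weight on an on-demand scan actor carrying scan and glitch materials.
; Looping timers randomize the glitch parameters.
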(event `self.ReceiveBeginPlay`
  (bind _asplayer_controller (cast `PlayerController` (`self.GetOwner`))
    (:`then`
      (set `self.PlayerController` _asplayer_controller)
      (`self.UpdateScanState` "NewEnumerator3" true)
      (`KismetMaterialLibrary.SetScalarParameterValue` "/Game/A_Mask/ScanComponent/VFX/SceneScan/Material/MPC/MPC_ScanParam.MPC_ScanParam" "GridCellSize" (`self.Grid Cell Size`))
      (`KismetMaterialLibrary.SetScalarParameterValue` "/Game/A_Mask/ScanComponent/VFX/SceneScan/Material/MPC/MPC_ScanParam.MPC_ScanParam" "MaxScanRange" (`self.MaxScanRange`)))
    (:`CastFailed`
      (`self.UpdateScanState` "NewEnumerator4" true))))

(event `self.ReceiveTick`
  (params (DeltaSeconds :type "Float (single-precision)"))
  (`self.UpdateScanTime` DeltaSeconds)
  (switch `/Game/A_Mask/ScanComponent/VFX/SceneScan/Enum/EBP_ScanState` (`self.GetScanState`)
    (:`NewEnumerator0`
      (`self.UpdateScanPPBlendWeight` :!label _label))
    (:`NewEnumerator1`
      _)
    (:`NewEnumerator2`
      (goto _label))
    (:`NewEnumerator3`
      _))
  (`self.UpdateScanLocation`)
  (bind _asbp_mask_player (cast `/Game/A_Mask/Character/Player/BP_MaskPlayer` (`GameplayStatics.GetPlayerCharacter` 0)))
  (`CameraComponent.SetFieldOfView` (`/Game/A_Mask/Character/BP_MaskCharacter_Base.FollowCamera` _asbp_mask_player) (`CurveFloat.GetFloatValue` (`self.CamFOVCurve`) (`self.ScanNormalizedTime`)))
  ;[1 1 1] Set Material Parameters
  (`/Engine/EditorBlueprintResources/StandardMacros.DoOnce` false
    (:`Completed`
      (`KismetSystemLibrary.K2_SetTimerDelegate` (delegate `RNGPerTime_1`) (`self.GlitchDuration`) true)
      (`KismetSystemLibrary.K2_SetTimerDelegate` (delegate `RNGPerTime_2`) (+ 0.2 (`self.GlitchDuration`)) true)
      (`KismetSystemLibrary.K2_SetTimerDelegate` (delegate `RNGPerTime_3`) 1.0 true))))

(event `RNGPerTime_3`
  (bind _returnvalue (`KismetMathLibrary.RandomFloatInRange` -0.05 0.05))
  (bind _hglitchmid (`self.HGlitchMID`))
  (bind _hglitchmid_2 (`self.HGlitchMID`))
  ;[1 1 1] Set Material Parameters
  (if (`KismetMathLibrary.RandomBoolWithWeight` 0.15)
    (`MaterialInstanceDynamic.SetScalarParameterValue` _hglitchmid_2 "HorizontalGlitchSlices" (`KismetMathLibrary.Conv_IntToDouble` (`KismetMathLibrary.RandomIntegerInRange` 4 10)))
    (`MaterialInstanceDynamic.SetScalarParameterValue` _hglitchmid_2 "Hue Separation Intensity" _returnvalue)
    (`MaterialInstanceDynamic.SetScalarParameterValue` _hglitchmid "Horizontal Glitch Intensity" _returnvalue)
    (`KismetSystemLibrary.Delay` (`KismetMathLibrary.RandomFloatInRange` 0.05 0.2))
    (`MaterialInstanceDynamic.SetScalarParameterValue` _hglitchmid "Horizontal Glitch Intensity" 0.0)
    (`MaterialInstanceDynamic.SetScalarParameterValue` _hglitchmid "Hue Separation Intensity" 0.0)))

(event `RNGPerTime_1`
  ;[1 1 1] Set Material Parameters
  (`KismetMaterialLibrary.SetScalarParameterValue` "/Game/A_Mask/ScanComponent/VFX/SceneScan/Material/MPC/MPC_ScanParam.MPC_ScanParam" "Ranom01" (`KismetMathLibrary.RandomFloatInRange` 0.0 1.0))
  (`MaterialInstanceDynamic.SetScalarParameterValue` (`self.GlitchMID`) "Voxel Size" (`KismetMathLibrary.Conv_IntToDouble` (`KismetMathLibrary.RandomIntegerInRange` 5 10))))

(event `RNGPerTime_2`
  ;[1 1 1] Set Material Parameters
  (`KismetMaterialLibrary.SetScalarParameterValue` "/Game/A_Mask/ScanComponent/VFX/SceneScan/Material/MPC/MPC_ScanParam.MPC_ScanParam" "Ranom01" (`KismetMathLibrary.RandomFloatInRange` 0.0 1.0))
  (`MaterialInstanceDynamic.SetScalarParameterValue` (`self.GlitchMID`) "Voxel Size" (`KismetMathLibrary.Conv_IntToDouble` (`KismetMathLibrary.RandomIntegerInRange` 5 10))))

(fn `DestroyPPActor`
  (bind _scan_actor (`self.Scan Actor`))
  (if (and (`KismetSystemLibrary.IsValid` _scan_actor) (`self.bDestroyActor`))
    (`Actor.K2_DestroyActor` _scan_actor)
    (set `self.Scan Actor` null)))

(fn `EndScan`
  (returns (bEnded :type Boolean))
  (switch `/Game/A_Mask/ScanComponent/VFX/SceneScan/Enum/EBP_ScanState` (`self.GetScanState`)
    (:`NewEnumerator0`
      _)
    (:`NewEnumerator1`
      _)
    (:`NewEnumerator2`
      (return false))
    (:`NewEnumerator3`
      (return false))
    (:`NewEnumerator4`
      (return false)))
  (bind _bupdated (`self.UpdateScanState` "NewEnumerator2"))
  (return _bupdated))

(fn `GetScanPPActor`
  (returns (ScanActor :type "/Game/A_Mask/ScanComponent/VFX/SceneScan/Blueprints/BP_ScanActor Object Reference"))
  (bind _glitchmaterial (`self.GlitchMaterial`))
  (bind _ppmaterial (`self.PPMaterial`))
  (bind _hglitchmaterial (`self.HGlitchMaterial`))
  (bind _postprocess (`/Game/A_Mask/ScanComponent/VFX/SceneScan/Blueprints/BP_ScanActor.PostProcess` (`self.Scan Actor`)))
  (`/Engine/EditorBlueprintResources/StandardMacros.IsValid` (`self.Scan Actor`)
    (:`Is Valid`
      (return (stale _output_get)))
    (:`Is Not Valid`
      (bind _returnvalue (`|SpawnActorFromClass` "/Game/A_Mask/ScanComponent/VFX/SceneScan/Blueprints/BP_ScanActor.BP_ScanActor_C" (`KismetMathLibrary.MakeTransform` (0.0 0.0 0.0)) "Undefined" "MultiplyWithRoot" null null))
      (bind _output_get (set `self.Scan Actor` _returnvalue))
      (`|ExecutionSequence`
        (:`then_0`
          (`/Engine/EditorBlueprintResources/StandardMacros.IsValid` (`self.PPMID`)
            (:`Is Valid`
              _)
            (:`Is Not Valid`
              (`/Engine/EditorBlueprintResources/StandardMacros.IsValid` _ppmaterial
                (:`Is Valid`
                  (bind _returnvalue_2 (`KismetMaterialLibrary.CreateDynamicMaterialInstance` _ppmaterial))
                  (set `self.PPMID` _returnvalue_2)))))
          (`/Engine/EditorBlueprintResources/StandardMacros.IsValid` _postprocess
            (:`Is Valid`
              (`PostProcessComponent.AddOrUpdateBlendable` _postprocess (`self.PPMID`) 1.0))))
        (:`then_1`
          (`/Engine/EditorBlueprintResources/StandardMacros.IsValid` (`self.GlitchMID`)
            (:`Is Valid`
              _)
            (:`Is Not Valid`
              (`/Engine/EditorBlueprintResources/StandardMacros.IsValid` _glitchmaterial
                (:`Is Valid`
                  (bind _returnvalue_3 (`KismetMaterialLibrary.CreateDynamicMaterialInstance` _glitchmaterial))
                  (set `self.GlitchMID` _returnvalue_3)))))
          (`PostProcessComponent.AddOrUpdateBlendable` (`/Game/A_Mask/ScanComponent/VFX/SceneScan/Blueprints/BP_ScanActor.PostProcess` (`self.Scan Actor`)) (`self.GlitchMID`) 1.0))
        (:`then_2`
          (`/Engine/EditorBlueprintResources/StandardMacros.IsValid` (`self.HGlitchMID`)
            (:`Is Valid`
              _)
            (:`Is Not Valid`
              (`/Engine/EditorBlueprintResources/StandardMacros.IsValid` _hglitchmaterial
                (:`Is Valid`
                  (bind _returnvalue_4 (`KismetMaterialLibrary.CreateDynamicMaterialInstance` _hglitchmaterial))
                  (set `self.HGlitchMID` _returnvalue_4)))))
          (`PostProcessComponent.AddOrUpdateBlendable` (`/Game/A_Mask/ScanComponent/VFX/SceneScan/Blueprints/BP_ScanActor.PostProcess` (`self.Scan Actor`)) (`self.HGlitchMID`) 1.0))
        (:`then_3`
          (return _output_get))))))

(fn `GetScanState`
  (returns (State :type "/Game/A_Mask/ScanComponent/VFX/SceneScan/Enum/EBP_ScanState Enum"))
  (return (`self.State`)))

(fn `StartScan`
  (returns (bStarted :type Boolean))
  (switch `/Game/A_Mask/ScanComponent/VFX/SceneScan/Enum/EBP_ScanState` (`self.GetScanState`)
    (:`NewEnumerator0`
      _)
    (:`NewEnumerator1`
      _)
    (:`NewEnumerator2`
      (bind _bupdated (`self.UpdateScanState` "NewEnumerator0" :!label _label))
      (return _bupdated))
    (:`NewEnumerator3`
      (goto _label))
    (:`NewEnumerator4`
      _))
  (return false))

(fn `UpdateScanLocation`
  (locals (ThisLocation :type "Vector Structure" :default (0.0 0.0 0.0)))
  (bind _playercontroller (`self.PlayerController`))
  (bind _returnvalue (`Controller.K2_GetPawn` _playercontroller))
  (`/Engine/EditorBlueprintResources/StandardMacros.IsValid` _playercontroller
    (:`Is Valid`
      (`/Engine/EditorBlueprintResources/StandardMacros.IsValid` _returnvalue
        (:`Is Valid`
          (bind _output_get (set `local.ThisLocation` (`Actor.K2_GetActorLocation` _returnvalue)))
          (`KismetMaterialLibrary.SetVectorParameterValue` "/Game/A_Mask/ScanComponent/VFX/SceneScan/Material/MPC/MPC_ScanParam.MPC_ScanParam" "Location" (`KismetMathLibrary.Conv_VectorToLinearColor` _output_get)))))))

(fn `UpdateScanPPBlendWeight`
  (locals (ThisTime :type "Float (double-precision)"))
  (bind _ppblendcurve (`self.PPBlendCurve`))
  (bind _scannormalizedtime (`self.ScanNormalizedTime`))
  (`/Engine/EditorBlueprintResources/StandardMacros.IsValid` _ppblendcurve
    (:`Is Valid`
      (set `local.ThisTime` (`CurveFloat.GetFloatValue` _ppblendcurve _scannormalizedtime)))
    (:`Is Not Valid`
      (set `local.ThisTime` _scannormalizedtime)))
  (bind _scanactor (`self.GetScanPPActor`))
  (`/Engine/EditorBlueprintResources/StandardMacros.IsValid` _scanactor
    (:`Is Valid`
      (bind _postprocess (`/Game/A_Mask/ScanComponent/VFX/SceneScan/Blueprints/BP_ScanActor.PostProcess` _scanactor))
      (`/Engine/EditorBlueprintResources/StandardMacros.IsValid` _postprocess
        (:`Is Valid`
          (set `PostProcessComponent.BlendWeight` (`local.ThisTime`) _postprocess))))))

(fn `UpdateScanState`
  (params (State :type "/Game/A_Mask/ScanComponent/VFX/SceneScan/Enum/EBP_ScanState Enum" :default "NewEnumerator0") (bForce :type Boolean))
  (returns (bUpdated :type Boolean))
  (if (or (`|EnumInequality` State (`self.State`)) bForce)
    (`|ExecutionSequence`
      (:`then_0`
        (switch `/Game/A_Mask/ScanComponent/VFX/SceneScan/Enum/EBP_ScanState` (`self.State`) ; Exit current state
          (:`NewEnumerator1`
            (`KismetMaterialLibrary.SetScalarParameterValue` "/Game/A_Mask/ScanComponent/VFX/SceneScan/Material/MPC/MPC_ScanParam.MPC_ScanParam" "bFadedIn"))
          (:`NewEnumerator3`
            (`KismetMaterialLibrary.SetScalarParameterValue` "/Game/A_Mask/ScanComponent/VFX/SceneScan/Material/MPC/MPC_ScanParam.MPC_ScanParam" "bFadedOut")
            (`self.SetComponentTickEnabled` true))))
      (:`then_1`
        (bind _output_get (set `self.State` State))
        (switch `/Game/A_Mask/ScanComponent/VFX/SceneScan/Enum/EBP_ScanState` _output_get ; Enter new state
          (:`NewEnumerator1`
            (`KismetMaterialLibrary.SetScalarParameterValue` "/Game/A_Mask/ScanComponent/VFX/SceneScan/Material/MPC/MPC_ScanParam.MPC_ScanParam" "bFadedIn" 1.0)
            (`self.UpdateScanPPBlendWeight`))
          (:`NewEnumerator3`
            (`KismetMaterialLibrary.SetScalarParameterValue` "/Game/A_Mask/ScanComponent/VFX/SceneScan/Material/MPC/MPC_ScanParam.MPC_ScanParam" "bFadedOut" 1.0)
            (`self.UpdateScanPPBlendWeight`)
            (`|ExecutionSequence`
              (:`then_1`
                (`self.SetComponentTickEnabled` false :!label _label)
                (`self.DestroyPPActor`))))
          (:`NewEnumerator4`
            (goto _label))))
      (:`then_2`
        (return true)))
    (else
      (return false))))

(fn `UpdateScanTime`
  (params (DeltaTime :type "Float (double-precision)"))
  (returns (bUpdated :type Boolean))
  (`|ExecutionSequence`
    (:`then_0`
      (switch `/Game/A_Mask/ScanComponent/VFX/SceneScan/Enum/EBP_ScanState` (`self.GetScanState`)
        (:`NewEnumerator0`
          (bind _output_get (set `self.ScanNormalizedTime` (+ (`self.ScanNormalizedTime`) (* (`local.DeltaTime`) (`self.FadeInSpeed`)))))
          (if (>= _output_get 1.0)
            (set `self.ScanNormalizedTime` 1.0)
            (`self.UpdateScanState` "NewEnumerator1")))
        (:`NewEnumerator2`
          (bind _output_get_2 (set `self.ScanNormalizedTime` (- (`self.ScanNormalizedTime`) (* (`local.DeltaTime`) (`self.FadeOutSpeed`)))))
          (if (<= _output_get_2 0.0)
            (set `self.ScanNormalizedTime` 0.0)
            (`self.UpdateScanState` "NewEnumerator3")))
        (:`NewEnumerator4`
          (return false)))
      (`KismetMaterialLibrary.SetScalarParameterValue` "/Game/A_Mask/ScanComponent/VFX/SceneScan/Material/MPC/MPC_ScanParam.MPC_ScanParam" "NormalizedTime" (`self.ScanNormalizedTime`)))
    (:`then_1`
      (return true))))