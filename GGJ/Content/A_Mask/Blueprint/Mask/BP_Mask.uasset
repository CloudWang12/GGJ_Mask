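; BP_Mask is a mask pickup actor that the player can collect to change masks.
; The construction script sets its mesh from the DT_Mask row matching its ID.
; Each tick the mesh yaws to face the player, and capsule overlap with BP_MaskPlayer toggles an interact flag.
; When InteractwithPlayer fires while that flag is set, it passes its ID to the player's ChangeMask and destroys itself.
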(event `self.ReceiveBeginPlay`)

(event `self.ReceiveTick`
  (params (DeltaSeconds :type "Float (single-precision)"))
  (bind (_returnvalue_roll _returnvalue_pitch _returnvalue_yaw) (`KismetMathLibrary.BreakRotator` (`KismetMathLibrary.FindLookAtRotation` (`self.K2_GetActorLocation`) (`self.K2_GetActorLocation` (`GameplayStatics.GetPlayerPawn` 0)))))
  (`SceneComponent.K2_SetWorldRotation` (`self.MaskMesh`) (`KismetMathLibrary.MakeRotator` 0.0 0.0 _returnvalue_yaw) false false))

(event `self.Capsule.OnComponentBeginOverlap`
  (params (OverlappedComponent :type "PrimitiveComponent Object Reference") (OtherActor :type "Actor Object Reference") (OtherComp :type "PrimitiveComponent Object Reference") (OtherBodyIndex :type Integer) (bFromSweep :type Boolean) (SweepResult :type "HitResult Structure (by ref)"))
  (cast `/Game/A_Mask/Character/Player/BP_MaskPlayer` OtherActor)
  (set `self.bInteract` true))

(event `self.Capsule.OnComponentEndOverlap`
  (params (OverlappedComponent :type "PrimitiveComponent Object Reference") (OtherActor :type "Actor Object Reference") (OtherComp :type "PrimitiveComponent Object Reference") (OtherBodyIndex :type Integer))
  (cast `/Game/A_Mask/Character/Player/BP_MaskPlayer` OtherActor)
  (set `self.bInteract` false))

(event `/Game/A_Mask/Blueprint/Interface/BPI_Interact.InteractWithPlayer`
  (if (`self.bInteract`)
    (bind _asbp_mask_player (cast `/Game/A_Mask/Character/Player/BP_MaskPlayer` (`GameplayStatics.GetPlayerPawn` 0)))
    (`/Game/A_Mask/Character/Player/BP_MaskPlayer.ChangeMask` _asbp_mask_player (`self.ID`))
    (`self.K2_DestroyActor`)))

(fn `UserConstructionScript`
  (bind _returnvalue (`|GetDataTableRow` "/Game/A_Mask/Data/DT_Mask.DT_Mask" (`self.ID`))
    (:`then`
      (`StaticMeshComponent.SetStaticMesh` (`self.MaskMesh`) (`.MaskMesh_27_583EB032477B8E2A0D4E13A1701B7E3D` (break `/Game/A_Mask/Data/S_Mask` _returnvalue))))))