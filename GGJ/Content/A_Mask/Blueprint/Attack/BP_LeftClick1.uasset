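; BP_LeftClick1 is a short-lived attack actor, apparently for the mask's left-click attack, that damages NPCs it overlaps.
; On BeginPlay it looks up MaskID in DT_Mask, applies that row's Niagara template, and destroys itself after a brief delay.
; AttackSphere overlaps with BP_NPC_Base apply the row's attack value as damage and pass a value derived from the result to BP_Health's HealthChange.
; The Box hit event is an empty override.
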(event `self.Box.OnComponentHit`
  (params (HitComponent :type "PrimitiveComponent Object Reference") (OtherActor :type "Actor Object Reference") (OtherComp :type "PrimitiveComponent Object Reference") (NormalImpulse :type "Vector Structure") (Hit :type "HitResult Structure (by ref)"))
  ; 继承父类必须重写
)

(event `self.ReceiveBeginPlay`
  (bind _returnvalue (`|GetDataTableRow` "/Game/A_Mask/Data/DT_Mask.DT_Mask" (`self.MaskID`))
    (:`then`
      (`NiagaraComponent.SetAsset` (`self.Niagara`) (`.NiagaraTemplate_35_EED81E3246C48CB2273504BDED7162AC` (break `/Game/A_Mask/Data/S_Mask` _returnvalue)) true)
      (`KismetSystemLibrary.Delay` 1.0)
      (`self.K2_DestroyActor`))))

(event `self.AttackSphere.OnComponentBeginOverlap`
  (params (OverlappedComponent :type "PrimitiveComponent Object Reference") (OtherActor :type "Actor Object Reference") (OtherComp :type "PrimitiveComponent Object Reference") (OtherBodyIndex :type Integer) (bFromSweep :type Boolean) (SweepResult :type "HitResult Structure (by ref)"))
  (bind _asbp_npc_base (cast `/Game/A_Mask/Character/AI/BP_NPC_Base` OtherActor))
  (bind _returnvalue (`GameplayStatics.ApplyDamage` _asbp_npc_base (`.AttackValue_18_9EEE94F0445E62CC400F81A2FB2A2D0F` (break `/Game/A_Mask/Data/S_Mask` (stale `self.ReceiveBeginPlay` _returnvalue)))))
  (bind _result (`/Engine/EditorBlueprintResources/StandardMacros.NegateFloat` _returnvalue)
    (:`  `
      (`/Game/A_Mask/Blueprint/Component/BP_Health.HealthChange` (`self.GetComponentByClass` _asbp_npc_base "/Game/A_Mask/Blueprint/Component/BP_Health.BP_Health_C") _result))))

(fn `UserConstructionScript`
  (`parent.UserConstructionScript`))