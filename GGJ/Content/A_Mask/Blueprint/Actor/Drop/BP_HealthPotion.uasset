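; BP_HealthPotion is a health pickup actor that changes the player's health when the player interacts with it.
; The InteractwithPlayer event casts the player pawn to BP_MaskPlayer and passes its AddHealth value to HealthChange on the player's HealthComponent.
; It then destroys itself and prints the player's resulting health as debug output.
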(event `/Game/A_Mask/Blueprint/Interface/BPI_Interact.InteractWithPlayer`
  (bind _asbp_mask_player (cast `/Game/A_Mask/Character/Player/BP_MaskPlayer` (`GameplayStatics.GetPlayerPawn` 0)))
  (bind _healthcomponent (`/Game/A_Mask/Character/Player/BP_MaskPlayer.HealthComponent` _asbp_mask_player))
  (`/Game/A_Mask/Blueprint/Component/BP_Health.HealthChange` _healthcomponent (`self.AddHealth`))
  (`self.K2_DestroyActor`)
  (`KismetSystemLibrary.PrintString` (`KismetStringLibrary.Conv_DoubleToString` (`/Game/A_Mask/Blueprint/Component/BP_Health.Health` _healthcomponent))))

(fn `UserConstructionScript`
  (`parent.UserConstructionScript`))