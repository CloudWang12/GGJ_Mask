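; BP_Mask is a mask pickup actor that changes the player's mask when interacted with.
; The construction script looks up its ID in DT_Mask and sets the mesh from that row.
; A sphere overlap shows or hides a widget while BP_MaskPlayer is in range.
; InteractwithPlayer passes the ID to the player's ChangeMask, then destroys the actor.
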(event `/Game/A_Mask/Blueprint/Interface/BPI_Interact.InteractWithPlayer`
  (bind _asbp_mask_player (cast `/Game/A_Mask/Character/Player/BP_MaskPlayer` (`GameplayStatics.GetPlayerPawn` 0)))
  (`/Game/A_Mask/Character/Player/BP_MaskPlayer.ChangeMask` _asbp_mask_player (`self.ID`))
  (`self.K2_DestroyActor`))

(event `self.Sphere.OnComponentBeginOverlap`
  (params (OverlappedComponent :type "PrimitiveComponent Object Reference") (OtherActor :type "Actor Object Reference") (OtherComp :type "PrimitiveComponent Object Reference") (OtherBodyIndex :type Integer) (bFromSweep :type Boolean) (SweepResult :type "HitResult Structure (by ref)"))
  (cast `/Game/A_Mask/Character/Player/BP_MaskPlayer` OtherActor)
  (`SceneComponent.SetVisibility` (`self.Widget`) true false))

(event `self.Sphere.OnComponentEndOverlap`
  (params (OverlappedComponent :type "PrimitiveComponent Object Reference") (OtherActor :type "Actor Object Reference") (OtherComp :type "PrimitiveComponent Object Reference") (OtherBodyIndex :type Integer))
  (cast `/Game/A_Mask/Character/Player/BP_MaskPlayer` OtherActor)
  (`SceneComponent.SetVisibility` (`self.Widget`) false false))

(fn `UserConstructionScript`
  (bind _returnvalue (`|GetDataTableRow` "/Game/A_Mask/Data/DT_Mask.DT_Mask" (`self.ID`))
    (:`then`
      (`StaticMeshComponent.SetStaticMesh` (`self.Mesh`) (`.MaskMesh_27_583EB032477B8E2A0D4E13A1701B7E3D` (break `/Game/A_Mask/Data/S_Mask` _returnvalue))))))