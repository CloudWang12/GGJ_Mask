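; BP_BossCameraArea is a trigger volume that stages the player's entry into a boss area.
; On overlap by a BP_MaskPlayer implementing BPI_BossCamera, it disables input and detaches the follow camera.
; For three seconds, Tick eases camera and player toward marker transforms with TInterpTo, teleporting the player.
; It then enables Box1's collision, sends InBossAreaMessage to the player and stops interpolating, without re-enabling input itself.
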(event `self.Box.OnComponentBeginOverlap`
  (params (OverlappedComponent :type "PrimitiveComponent Object Reference") (OtherActor :type "Actor Object Reference") (OtherComp :type "PrimitiveComponent Object Reference") (OtherBodyIndex :type Integer) (bFromSweep :type Boolean) (SweepResult :type "HitResult Structure (by ref)"))
  (bind _asbp_mask_player (cast `/Game/A_Mask/Character/Player/BP_MaskPlayer` OtherActor))
  (cast `/Game/A_Mask/Blueprint/Interface/BPI_BossCamera` _asbp_mask_player)
  (bind _output_get (set `self.As BP Mask Player` _asbp_mask_player))
  (`self.DisableInput` (`/Game/A_Mask/Character/Player/BP_MaskPlayer.MaskPlayerController` _output_get) null)
  (bind _output_get_2 (set `self.Follow Camera` (`/Game/A_Mask/Character/BP_MaskCharacter_Base.FollowCamera` _asbp_mask_player)))
  (`SceneComponent.K2_DetachFromComponent` _output_get_2 "KeepWorld" "KeepWorld" "KeepWorld" true)
  (set `self.bPlayerIn` true)
  (`KismetSystemLibrary.Delay` 3.0)
  (`PrimitiveComponent.SetCollisionEnabled` (`self.Box1`) "QueryAndPhysics")
  (message `/Game/A_Mask/Blueprint/Interface/BPI_BossCamera.InBossArea` (`self.As BP Mask Player`))
  (set `self.bPlayerIn` false))

(event `self.ReceiveTick`
  (params (DeltaSeconds :type "Float (single-precision)"))
  (if (`self.bPlayerIn`)
    (`SceneComponent.K2_SetWorldTransform` (`self.Follow Camera`) (`KismetMathLibrary.TInterpTo` (`SceneComponent.K2_GetComponentToWorld` (`self.Follow Camera`)) (`SceneComponent.K2_GetComponentToWorld` (`self.CameraLocation`)) DeltaSeconds 1.0) false false)
    (`self.K2_SetActorTransform` (`self.As BP Mask Player`) (`KismetMathLibrary.TInterpTo` (`self.GetTransform` (`self.As BP Mask Player`)) (`SceneComponent.K2_GetComponentToWorld` (`self.PlayerLocation`)) DeltaSeconds 1.0) false true)))

(fn `UserConstructionScript`)