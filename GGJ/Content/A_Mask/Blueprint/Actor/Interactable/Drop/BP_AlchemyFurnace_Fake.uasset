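; BP_AlchemyFurnace_Fake is a single-use interactable furnace that drops fake alchemy pills.
; A sphere overlap shows or hides its widget for BP_MaskPlayer, and Tick turns that widget's yaw toward the camera.
; On first interaction it sets Used, hides DropEffects, and spawns a small random number of BP_AlchemyPill_Fake actors at its Scene component's transform.
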(event `self.ReceiveBeginPlay`)

(event `self.ReceiveTick`
  (params (DeltaSeconds :type "Float (single-precision)"))
  (bind (_returnvalue_roll _returnvalue_pitch _returnvalue_yaw) (`KismetMathLibrary.BreakRotator` (`KismetMathLibrary.FindLookAtRotation` (`SceneComponent.K2_GetComponentLocation` (`self.Widget`)) (`self.K2_GetActorLocation` (`GameplayStatics.GetPlayerCameraManager` 0)))))
  (`SceneComponent.K2_SetRelativeRotation` (`self.Widget`) (`KismetMathLibrary.MakeRotator` 0.0 0.0 _returnvalue_yaw) false false))

(event `self.Sphere.OnComponentBeginOverlap`
  (params (OverlappedComponent :type "PrimitiveComponent Object Reference") (OtherActor :type "Actor Object Reference") (OtherComp :type "PrimitiveComponent Object Reference") (OtherBodyIndex :type Integer) (bFromSweep :type Boolean) (SweepResult :type "HitResult Structure (by ref)"))
  (cast `/Game/A_Mask/Character/Player/BP_MaskPlayer` OtherActor)
  (`SceneComponent.SetVisibility` (`self.Widget`) true false))

(event `self.Sphere.OnComponentEndOverlap`
  (params (OverlappedComponent :type "PrimitiveComponent Object Reference") (OtherActor :type "Actor Object Reference") (OtherComp :type "PrimitiveComponent Object Reference") (OtherBodyIndex :type Integer))
  (cast `/Game/A_Mask/Character/Player/BP_MaskPlayer` OtherActor)
  (`SceneComponent.SetVisibility` (`self.Widget`) false false))

(event `self.InteractWithPlayer`
  (if (not (`self.bUsed`))
    (set `self.bUsed` true)
    (`SceneComponent.SetVisibility` (`self.DropEffects`) false false)
    (for _ (range (+ (`KismetMathLibrary.RandomIntegerInRange` 0 4) 1))
      (`|SpawnActorFromClass` "/Game/A_Mask/Blueprint/Actor/Interactable/Drop/BP_AlchemyPill_Fake.BP_AlchemyPill_Fake_C" (`SceneComponent.K2_GetComponentToWorld` (`self.Scene`)) "AlwaysSpawn" "MultiplyWithRoot" null null))))

(fn `UserConstructionScript`)