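; BP_AlchemyPill is an alchemy pill drop that flies to the player and is collected on contact.
; On spawn, an impulse pops its physics Sphere upward in a random horizontal direction.
; After one second it hides the drop effect, shows the Trigger, stops physics and eases toward the player pawn each tick.
; Once moving, overlapping BP_MaskPlayer calls PickUpAlchemyPill and destroys the actor.
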(event `self.ReceiveBeginPlay`
  (bind (_x _y) (`KismetMathLibrary.BreakVector2D` (* (`KismetMathLibrary.Normal2D` (`KismetMathLibrary.MakeVector2D` (`KismetMathLibrary.RandomFloatInRange` -1.0 1.0) (`KismetMathLibrary.RandomFloatInRange` -1.0 1.0))) 200.0)))
  (`PrimitiveComponent.AddImpulse` (`self.Sphere`) (`KismetMathLibrary.MakeVector` _x _y 200.0) "None" true)
  (`KismetSystemLibrary.Delay` 1.0)
  (set `self.bCanMove` true)
  (`SceneComponent.SetVisibility` (`self.DropEffects`) false false)
  (`SceneComponent.SetVisibility` (`self.Trigger`) true false)
  (`PrimitiveComponent.SetSimulatePhysics` (`self.Sphere`) false))

(event `self.ReceiveTick`
  (params (DeltaSeconds :type "Float (single-precision)"))
  (if (`self.bCanMove`)
    (`SceneComponent.K2_SetWorldLocation` (`self.Sphere`) (`KismetMathLibrary.VInterpTo` (`SceneComponent.K2_GetComponentLocation` (`self.Sphere`)) (+ (`self.K2_GetActorLocation` (`GameplayStatics.GetPlayerPawn` 0)) (0.0 0.0 45.0)) DeltaSeconds 3.0) false false)))

(event `self.Trigger.OnComponentBeginOverlap`
  (params (OverlappedComponent :type "PrimitiveComponent Object Reference") (OtherActor :type "Actor Object Reference") (OtherComp :type "PrimitiveComponent Object Reference") (OtherBodyIndex :type Integer) (bFromSweep :type Boolean) (SweepResult :type "HitResult Structure (by ref)"))
  (if (`self.bCanMove`)
    (bind _asbp_mask_player (cast `/Game/A_Mask/Character/Player/BP_MaskPlayer` OtherActor))
    (`/Game/A_Mask/Character/Player/BP_MaskPlayer.PickUpAlchemyPill` _asbp_mask_player)
    (`self.K2_DestroyActor`)))

(fn `UserConstructionScript`
  (`parent.UserConstructionScript`))