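; BP_FlySword is a homing sword projectile, filed under boss skills, that chases its Enemy actor.
; Each tick it moves forward at Speed and turns toward Enemy, with the turn rate rising as the distance closes.
; Its Box overlap deals fixed damage to Enemy and destroys the sword, which also self-destructs when Enemy is invalid.
; Unconnected leftover nodes hold an unused delayed speed-up.
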(event `self.ReceiveTick`
  (params (DeltaSeconds :type "Float (single-precision)"))
  (bind _enemy (`self.Enemy`))
  (`/Engine/EditorBlueprintResources/StandardMacros.IsValid` _enemy
    (:`Is Valid`
      (`self.K2_SetActorLocationAndRotation` (+ (`self.K2_GetActorLocation`) (* (`self.GetActorForwardVector`) (`KismetMathLibrary.Conv_DoubleToVector` (* (`GameplayStatics.GetWorldDeltaSeconds`) (`self.Speed`))))) (`KismetMathLibrary.RInterpTo` (`self.K2_GetActorRotation`) (`KismetMathLibrary.FindLookAtRotation` (`self.K2_GetActorLocation`) (`self.K2_GetActorLocation` _enemy)) (`GameplayStatics.GetWorldDeltaSeconds`) (`self.SpeedOfSwordRotation`)))
      (set `self.SpeedOfSwordRotation` (`KismetMathLibrary.MapRangeClamped` (`KismetMathLibrary.Vector_Distance` (`self.K2_GetActorLocation`) (`self.K2_GetActorLocation` (`self.Enemy`))) 100.0 2000.0 100.0 5.0)))
    (:`Is Not Valid`
      (`self.K2_DestroyActor`))))

(event `self.Box.OnComponentBeginOverlap`
  (params (OverlappedComponent :type "PrimitiveComponent Object Reference") (OtherActor :type "Actor Object Reference") (OtherComp :type "PrimitiveComponent Object Reference") (OtherBodyIndex :type Integer) (bFromSweep :type Boolean) (SweepResult :type "HitResult Structure (by ref)"))
  (if (== OtherActor (`self.Enemy`))
    (`GameplayStatics.ApplyDamage` OtherActor 2.5)
    (`self.K2_DestroyActor`)))

(fn `UserConstructionScript`)