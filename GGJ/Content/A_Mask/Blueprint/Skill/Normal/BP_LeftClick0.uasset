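; BP_LeftClick0 is a left-click skill actor for the mask system, with visuals and damage driven by the DT_Mask row matching MaskID.
; On BeginPlay it looks up that row and assigns its left Niagara template.
; When its Box component hits something, it damages BP_NPC_Base actors by the row's attack value.
; Any hit spawns the row's impact effect, slightly offset along world X, then destroys the actor.
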(event `self.ReceiveBeginPlay`
  (bind _returnvalue (`|GetDataTableRow` "/Game/A_Mask/Data/DT_Mask.DT_Mask" (`self.MaskID`))
    (:`then`
      (`NiagaraComponent.SetAsset` (`self.Niagara`) (`.LeftNiagaraTemplate_51_EED81E3246C48CB2273504BDED7162AC` (break `/Game/A_Mask/Data/S_Mask` _returnvalue)) true))))

(event `self.Box.OnComponentHit`
  (params (HitComponent :type "PrimitiveComponent Object Reference") (OtherActor :type "Actor Object Reference") (OtherComp :type "PrimitiveComponent Object Reference") (NormalImpulse :type "Vector Structure") (Hit :type "HitResult Structure (by ref)"))
  (bind (_bblockinghit _binitialoverlap _time _distance _location _impactpoint _normal _impactnormal _physmat _hitactor) (`GameplayStatics.BreakHitResult` Hit))
  (bind _asbp_npc_base (cast `/Game/A_Mask/Character/AI/AI_Character/BP_NPC_Base` _hitactor)
    (:`then`
      (bind (_maskname _masktexture _attackvalue _uniquevalue _attacktexture _uniquetexture _uniquecooldown _maskcooldown _maskmesh _bp_normalattack _bp_ultimateattack _bp_surfaceworldskill _leftniagaratemplate _leftniagarahit) (break `/Game/A_Mask/Data/S_Mask` (stale `self.ReceiveBeginPlay` _returnvalue)))
      (`GameplayStatics.ApplyDamage` _asbp_npc_base _attackvalue))
    (:`CastFailed`
      _))
  (`NiagaraFunctionLibrary.SpawnSystemAtLocation` _leftniagarahit (`KismetMathLibrary.MakeVector` (- (.x _location) 18.0) (.y _location) (.z _location)))
  (`self.K2_DestroyActor`))

(fn `UserConstructionScript`)