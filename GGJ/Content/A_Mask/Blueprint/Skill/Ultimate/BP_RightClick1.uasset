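; BP_RightClick1 is a short-lived mask skill actor that damages and knocks back NPCs.
; On spawn it looks up its MaskID row in DT_Mask, applies that row's right-click Niagara effect and destroys itself after a second.
; AttackSphere overlaps deal triple the row's AttackValue to BP_NPC_Base actors.
; After a short shared delay, only the last stored NPC is launched up and away.
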(event `self.ReceiveBeginPlay`
  (bind _returnvalue (`|GetDataTableRow` "/Game/A_Mask/Data/DT_Mask.DT_Mask" (`self.MaskID`))
    (:`then`
      (`NiagaraComponent.SetAsset` (`self.Niagara`) (`.RightNiagaraTemplate_59_EACA76534FBA53ED3BF390BC91A1FE56` (break `/Game/A_Mask/Data/S_Mask` _returnvalue)) true)
      (`KismetSystemLibrary.Delay` 1.0)
      (`self.K2_DestroyActor`))))

(event `self.AttackSphere.OnComponentBeginOverlap`
  (params (OverlappedComponent :type "PrimitiveComponent Object Reference") (OtherActor :type "Actor Object Reference") (OtherComp :type "PrimitiveComponent Object Reference") (OtherBodyIndex :type Integer) (bFromSweep :type Boolean) (SweepResult :type "HitResult Structure (by ref)"))
  (bind (_returnvalue_x _returnvalue_y) (`KismetMathLibrary.BreakVector` (* (`KismetMathLibrary.Normal` (- (`self.K2_GetActorLocation` (`self.As BP NPC Base`)) (`self.K2_GetActorLocation`))) 1000.0)))
  (bind _asbp_npc_base (cast `/Game/A_Mask/Character/AI/AI_Character/BP_NPC_Base` OtherActor))
  (bind _output_get (set `self.As BP NPC Base` _asbp_npc_base))
  (`GameplayStatics.ApplyDamage` _output_get (* (`.AttackValue_18_9EEE94F0445E62CC400F81A2FB2A2D0F` (break `/Game/A_Mask/Data/S_Mask` (stale `self.ReceiveBeginPlay` _returnvalue))) 3.0))
  (`KismetSystemLibrary.Delay` 0.5)
  (`Character.LaunchCharacter` (`self.As BP NPC Base`) (`KismetMathLibrary.MakeVector` _returnvalue_x _returnvalue_y 500.0) true true))

(fn `UserConstructionScript`)