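; BP_RightClick2 is an ultimate-skill area actor that changes player health and damages NPCs inside its AttackSphere.
; The Buff timeline raises the per-second amount as it plays, then enables sphere physics and destroys the actor shortly after.
; Overlap timelines tick that amount into the player's HealthComponent or NPC damage, sharing one CurrentSecond counter with Buff.
; End overlap stops only the player's timeline.
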(event `self.ReceiveBeginPlay`
  (bind (_direction _hp) (`Timeline|Buff` :!via `PlayFromStart`)
    (:`Update`
      (if (>= (- _hp 1.0) (`self.CurrentSecond`))
        (set `self.CurrentSecond` (`KismetMathLibrary.FTrunc` _hp))
        (set `self.ChangeHPPreSecond` (+ (`self.ChangeHPPreSecond`) 1.0))))
    (:`Finished`
      (`PrimitiveComponent.SetSimulatePhysics` (`self.AttackSphere`) true)
      (`KismetSystemLibrary.Delay` 0.5)
      (`self.K2_DestroyActor`))))

(event `self.AttackSphere.OnComponentBeginOverlap`
  (params (OverlappedComponent :type "PrimitiveComponent Object Reference") (OtherActor :type "Actor Object Reference") (OtherComp :type "PrimitiveComponent Object Reference") (OtherBodyIndex :type Integer) (bFromSweep :type Boolean) (SweepResult :type "HitResult Structure (by ref)"))
  (bind _asbp_mask_player (cast `/Game/A_Mask/Character/Player/BP_MaskPlayer` OtherActor)
    (:`then`
      (bind (_direction _hp) (`Timeline|时间轴_0` :!via `PlayFromStart` :!label _label)
        (:`Update`
          (if (>= (- _hp 1.0) (`self.CurrentSecond`))
            (set `self.CurrentSecond` (`KismetMathLibrary.FTrunc` _hp))
            (`/Game/A_Mask/Blueprint/Component/BP_Health.HealthChange` (`/Game/A_Mask/Character/Player/BP_MaskPlayer.HealthComponent` _asbp_mask_player) (`self.ChangeHPPreSecond`))))))
    (:`CastFailed`
      (bind _asbp_npc_base (cast `/Game/A_Mask/Character/AI/AI_Character/BP_NPC_Base` OtherActor))
      (bind (_direction_2 _hp_2) (`Timeline|时间轴` :!via `PlayFromStart`)
        (:`Update`
          (if (>= (- _hp_2 1.0) (`self.CurrentSecond`))
            (set `self.CurrentSecond` (`KismetMathLibrary.FTrunc` _hp_2))
            (`GameplayStatics.ApplyDamage` _asbp_npc_base (`self.ChangeHPPreSecond`))))))))

(event `self.AttackSphere.OnComponentEndOverlap`
  (params (OverlappedComponent :type "PrimitiveComponent Object Reference") (OtherActor :type "Actor Object Reference") (OtherComp :type "PrimitiveComponent Object Reference") (OtherBodyIndex :type Integer))
  (cast `/Game/A_Mask/Character/Player/BP_MaskPlayer` OtherActor)
  (goto _label :!via `Stop`))

(fn `UserConstructionScript`)