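; BP_SurfaceSkill1 is a short-lived skill actor for a mask ability that breaks BP_BrokenWall obstacles.
; On BeginPlay it looks up MaskID in DT_Mask, applies that row's left Niagara template, then destroys itself after a brief delay.
; AttackSphere overlaps with a broken wall destroy only that wall's InnerWall actor, if valid.
; A hit-effect spawn using the row's left hit system is present but unconnected.
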(event `self.ReceiveBeginPlay`
  (bind _returnvalue (`|GetDataTableRow` "/Game/A_Mask/Data/DT_Mask.DT_Mask" (`self.MaskID`))
    (:`then`
      (`NiagaraComponent.SetAsset` (`self.Niagara`) (`.LeftNiagaraTemplate_51_EED81E3246C48CB2273504BDED7162AC` (break `/Game/A_Mask/Data/S_Mask` _returnvalue)) true)
      (`KismetSystemLibrary.Delay` 1.0)
      (`self.K2_DestroyActor`))))

(event `self.AttackSphere.OnComponentBeginOverlap`
  (params (OverlappedComponent :type "PrimitiveComponent Object Reference") (OtherActor :type "Actor Object Reference") (OtherComp :type "PrimitiveComponent Object Reference") (OtherBodyIndex :type Integer) (bFromSweep :type Boolean) (SweepResult :type "HitResult Structure (by ref)"))
  (bind _asbp_broken_wall (cast `/Game/A_Mask/Blueprint/Actor/Terrain/BP_BrokenWall` OtherActor))
  (bind _innerwall (`/Game/A_Mask/Blueprint/Actor/Terrain/BP_BrokenWall.InnerWall` _asbp_broken_wall))
  (`/Engine/EditorBlueprintResources/StandardMacros.IsValid` _innerwall
    (:`Is Valid`
      (`self.K2_DestroyActor` _innerwall))))

(fn `UserConstructionScript`)