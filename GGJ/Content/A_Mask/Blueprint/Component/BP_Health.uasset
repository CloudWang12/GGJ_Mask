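; BP_Health is a health component that stores a Health value bounded by MaxHealth.
; Its HealthChange function adds a signed delta to Health through nested branches, clamping the result between zero and MaxHealth.
; It fires no death or change notification, and its BeginPlay and Tick events are unused placeholders.
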(fn `HealthChange`
  (params (HealthChange :type "Float (double-precision)"))
  (bind _returnvalue (+ (`self.Health`) HealthChange))
  (if (<= _returnvalue 0.0)
    (set `self.Health` 0.0)
    (elif (> _returnvalue (`self.MaxHealth`))
      (set `self.Health` (`self.MaxHealth`))
      (else
        (set `self.Health` _returnvalue)))))