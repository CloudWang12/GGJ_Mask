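; Player character that switches between masks (default, Zhong Kui, Meng Po, Xie Bi'an), each changing its look, damage and abilities.
; ChangeMask pulls mesh, attack value and colour from DT_Mask and applies inner-world debuffs.
; NormalAttack, Ultimate and SurfaceWorldSkill branch on mask ID for DT_Mask-driven spawns, cursor-aimed attacks, teleport or temporary invulnerability.
; It also sphere-traces for interaction and mask pickups, and relays health and mask timers to the overlay HUD.
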(event `self.ReceiveBeginPlay`
  (`|ExecutionSequence`
    (:`then_0`
      (bind _asgi_mask (cast `/Game/A_Mask/Gameplay/GI_Mask` (`GameplayStatics.GetGameInstance`)))
      (set `self.GIMask` _asgi_mask))
    (:`then_1`
      (bind _returnvalue (`|CreateWidget` "/Game/A_Mask/Blueprint/UI/WBP_Overlay.WBP_Overlay_C"))
      (bind _output_get (set `self.WBP_Overlay` _returnvalue))
      (`UserWidget.AddToViewport` _output_get 0)
      (`self.HealthTargetPercentage`))
    (:`then_2`
      (bind _asbp_mask_player_state (cast `/Game/A_Mask/Gameplay/BP_MaskPlayerState` (`GameplayStatics.GetPlayerState` 0)))
      (set `self.MaskPlayerState` _asbp_mask_player_state))
    (:`then_3`
      (bind _asbp_mask_player_controller (cast `/Game/A_Mask/Gameplay/BP_MaskPlayerController` (`self.GetController`)))
      (set `self.MaskPlayerController` _asbp_mask_player_controller))
    (:`then_4`
      (set `self.CurrentSpeed` (`CharacterMovementComponent.MaxWalkSpeed` (`self.CharacterMovement`)))
      (set `self.NS Player` (`self.NS_Player`))
      (`self.ChangeMask` (`self.MaskID`) true))))

(event `self.ReceiveAnyDamage`
  (params (Damage :type "Float (single-precision)") (DamageType :type "DamageType Object Reference") (InstigatedBy :type "Controller Object Reference") (DamageCauser :type "Actor Object Reference"))
  (bind _returnvalue (* Damage (`self.DamageMultiplier`)))
  (bind _result (`/Engine/EditorBlueprintResources/StandardMacros.NegateFloat` _returnvalue)
    (:`  `
      (`/Game/A_Mask/Blueprint/Component/BP_Health.HealthChange` (`self.HealthComponent`) _result)
      (`self.HealthTargetPercentage`)
      (`KismetSystemLibrary.PrintString` (`KismetStringLibrary.Concat_StrStr` "BP_Player里的:" (`KismetSystemLibrary.GetDisplayName` self) "受到了" (`KismetStringLibrary.Conv_DoubleToString` _returnvalue) "伤害,剩下" (`KismetStringLibrary.Conv_DoubleToString` (`/Game/A_Mask/Blueprint/Component/BP_Health.Health` (`self.HealthComponent`))) "滴血") true true (struct :`R` 0.013707 :`G` 0.053062 :`B` 1.0 :`A` 1.0)))))

(event `EnhancedInput|/Game/A_Mask/Input/Actions/IA_Interact`
  (params (ActionValue :type Boolean) (ElapsedSeconds :type "Float (double-precision)") (TriggeredSeconds :type "Float (double-precision)") (InputAction :type "InputAction Object Reference" :default "/Game/A_Mask/Input/Actions/IA_Interact.IA_Interact"))
  (bind _capsulecomponent (`self.CapsuleComponent`))
  (bind _returnvalue (+ (`SceneComponent.K2_GetComponentLocation` _capsulecomponent) (0.0 0.0 50.0)))
  ; 射线检测
  (:`Started`
    (bind (_outhit _returnvalue_2) (`KismetSystemLibrary.SphereTraceSingle` _returnvalue (+ _returnvalue (* (`SceneComponent.GetForwardVector` _capsulecomponent) 100.0)) 100.0 "TraceTypeQuery1"))
    (if _returnvalue_2
      (bind (_bblockinghit _binitialoverlap _time _distance _location _impactpoint _normal _impactnormal _physmat _hitactor) (`GameplayStatics.BreakHitResult` _outhit))
      (bind _asbp_mask (cast `/Game/A_Mask/Blueprint/Actor/Interactable/Mask/BP_Mask` _hitactor)
        (:`then`
          (`BlueprintMapLibrary.Map_Add` (`self.IsMaskOKID`) (`/Game/A_Mask/Blueprint/Actor/Interactable/Mask/BP_Mask.ID` _asbp_mask) true)
          (message `/Game/A_Mask/Blueprint/Interface/BPI_Interact.InteractWithPlayer` _hitactor))
        (:`CastFailed`
          (message `/Game/A_Mask/Blueprint/Interface/BPI_Interact.InteractWithPlayer` _hitactor))))))

(fn `BackToDefaultStatus`
  (set `CharacterMovementComponent.MaxWalkSpeed` (`self.CurrentSpeed`) (`self.CharacterMovement`))
  (set `self.DamageMultiplier` 1.0)
  (set `self.bCanBeAttack` true))

(fn `ChangeMask`
  (params (MaskID :type Name) (IsOriginMask :type Boolean))
  (bind _output_get (set `self.MaskID` MaskID))
  (`|ExecutionSequence`
    (:`then_0`
      (bind _returnvalue (`|GetDataTableRow` "/Game/A_Mask/Data/DT_Mask.DT_Mask" _output_get)
        (:`then`
          (bind (_maskname _masktexture _attackvalue _uniquevalue _attacktexture _uniquetexturebackground _uniquetexturefill _maskmesh _bp_normalattack _bp_ultimateattack _bp_surfaceworldskill _leftniagaratemplate _leftniagarahit _playercolor) (break `/Game/A_Mask/Data/S_Mask` _returnvalue))
          (`StaticMeshComponent.SetStaticMesh` (`self.Mask`) _maskmesh)
          (set `/Game/A_Mask/Gameplay/BP_MaskPlayerState.NormalAttackDamage` _attackvalue (`self.MaskPlayerState`))
          (bind _output_get_2 (set `self.Player Color` _playercolor))
          (`NiagaraComponent.SetVariableLinearColor` (`self.NS Player`) "Color" _output_get_2))))
    (:`then_1`
      (switch `name` _output_get
        (:`0`
          (set `self.bMasking` false)
          (`self.BackToDefaultStatus`))
        (:`1`
          (if (`/Game/A_Mask/Gameplay/GI_Mask.bInnerWorld` (`self.GIMask`))
            ;[0.15 0.007162 0 0.5] 速度0.5x(钟馗DEBUFF)
            (set `CharacterMovementComponent.MaxWalkSpeed` (* (`self.CurrentSpeed`) 0.5) (`self.CharacterMovement`))))
        (:`2`
          (if (`/Game/A_Mask/Gameplay/GI_Mask.bInnerWorld` (`self.GIMask`))
            _))
        (:`3`
          (if (`/Game/A_Mask/Gameplay/GI_Mask.bInnerWorld` (`self.GIMask`))
            ;[0.15 0.007162 0 0.5] 受伤倍率2x(谢必安DEBUFF)
            (set `self.DamageMultiplier` 2.0)))))))

(fn `ClearMaskCD_MENGPO`
  (bind _wbp_overlay (`self.WBP_Overlay`))
  (bind _wbp_mask_mp (`/Game/A_Mask/Blueprint/UI/WBP_Overlay.WBP_Mask_MP` _wbp_overlay))
  ; Comment
  (`/Engine/EditorBlueprintResources/StandardMacros.IsValid` _wbp_overlay
    (:`Is Valid`
      (`/Engine/EditorBlueprintResources/StandardMacros.IsValid` _wbp_mask_mp
        (:`Is Valid`
          (`/Game/A_Mask/Blueprint/UI/SubWidget/WBP_Mask_MP.ClearMaskCD` _wbp_mask_mp))))))

(fn `ClearMaskCD_XBA`
  (bind _wbp_overlay (`self.WBP_Overlay`))
  (bind _wbp_mask_xba (`/Game/A_Mask/Blueprint/UI/WBP_Overlay.WBP_Mask_XBA` _wbp_overlay))
  ; Comment
  (`/Engine/EditorBlueprintResources/StandardMacros.IsValid` _wbp_overlay
    (:`Is Valid`
      (`/Engine/EditorBlueprintResources/StandardMacros.IsValid` _wbp_mask_xba
        (:`Is Valid`
          (`/Game/A_Mask/Blueprint/UI/SubWidget/WBP_Mask_XBA.ClearMaskCD` _wbp_mask_xba))))))

(fn `ClearMaskCD_ZHONGKUI`
  (bind _wbp_overlay (`self.WBP_Overlay`))
  (bind _wbp_mask_zk (`/Game/A_Mask/Blueprint/UI/WBP_Overlay.WBP_Mask_ZK` _wbp_overlay))
  ; Comment
  (`/Engine/EditorBlueprintResources/StandardMacros.IsValid` _wbp_overlay
    (:`Is Valid`
      (`/Engine/EditorBlueprintResources/StandardMacros.IsValid` _wbp_mask_zk
        (:`Is Valid`
          (`/Game/A_Mask/Blueprint/UI/SubWidget/WBP_Mask_ZK.ClearMaskCD` _wbp_mask_zk))))))

(fn `ClearMaskTime_MENGPO`
  (bind _wbp_overlay (`self.WBP_Overlay`))
  (bind _wbp_mask_mp (`/Game/A_Mask/Blueprint/UI/WBP_Overlay.WBP_Mask_MP` _wbp_overlay))
  ; Comment
  (`/Engine/EditorBlueprintResources/StandardMacros.IsValid` _wbp_overlay
    (:`Is Valid`
      (`/Engine/EditorBlueprintResources/StandardMacros.IsValid` _wbp_mask_mp
        (:`Is Valid`
          (`/Game/A_Mask/Blueprint/UI/SubWidget/WBP_Mask_MP.ClearMaskTime` _wbp_mask_mp))))))

(fn `ClearMaskTime_XBA`
  (bind _wbp_overlay (`self.WBP_Overlay`))
  (bind _wbp_mask_xba (`/Game/A_Mask/Blueprint/UI/WBP_Overlay.WBP_Mask_XBA` _wbp_overlay))
  ; Comment
  (`/Engine/EditorBlueprintResources/StandardMacros.IsValid` _wbp_overlay
    (:`Is Valid`
      (`/Engine/EditorBlueprintResources/StandardMacros.IsValid` _wbp_mask_xba
        (:`Is Valid`
          (`/Game/A_Mask/Blueprint/UI/SubWidget/WBP_Mask_XBA.ClearMaskTime` _wbp_mask_xba))))))

(fn `ClearMaskTime_ZHONGKUI`
  (bind _wbp_overlay (`self.WBP_Overlay`))
  (bind _wbp_mask_zk (`/Game/A_Mask/Blueprint/UI/WBP_Overlay.WBP_Mask_ZK` _wbp_overlay))
  ; Comment
  (`/Engine/EditorBlueprintResources/StandardMacros.IsValid` _wbp_overlay
    (:`Is Valid`
      (`/Engine/EditorBlueprintResources/StandardMacros.IsValid` _wbp_mask_zk
        (:`Is Valid`
          (`/Game/A_Mask/Blueprint/UI/SubWidget/WBP_Mask_ZK.ClearMaskTime` _wbp_mask_zk))))))

(fn `EatAlchemyPill`
  (if (< (`self.GourdNum`) (`self.MaxGourdNum`))
    (`/Engine/EditorBlueprintResources/StandardMacros.IncrementInt` (`self.GourdNum`))))

(fn `HealthTargetPercentage`
  (bind _wbp_overlay (`self.WBP_Overlay`))
  (bind _wbp_playerhealthbar (`/Game/A_Mask/Blueprint/UI/WBP_Overlay.WBP_PlayerHealthBar` _wbp_overlay))
  (`/Engine/EditorBlueprintResources/StandardMacros.IsValid` _wbp_overlay
    (:`Is Valid`
      (`/Engine/EditorBlueprintResources/StandardMacros.IsValid` _wbp_playerhealthbar
        (:`Is Valid`
          (set `/Game/A_Mask/Blueprint/UI/SubWidget/WBP_PlayerHealthBar.TargetPercentage` (`/Game/A_Mask/Blueprint/Component/BP_Health.GetHealthPercentage` (`self.HealthComponent`)) _wbp_playerhealthbar))))))

(fn `NormalAttack`
  (locals (SpawnRotation :type "Rotator Structure") (SpawnLocation :type "Vector Structure"))
  (bind (_returnvalue_location _returnvalue_rotation) (`KismetMathLibrary.BreakTransform` (`self.GetTransform`)))
  (bind (_returnvalue_roll _returnvalue_pitch) (`KismetMathLibrary.BreakRotator` (`self.K2_GetActorRotation`)))
  (bind (_returnvalue_location_2 _returnvalue_rotation_2) (`KismetMathLibrary.BreakTransform` (`self.GetTransform`)))
  (bind (_spawnrotation_roll _spawnrotation_pitch _spawnrotation_yaw) (`KismetMathLibrary.BreakRotator` (`local.SpawnRotation`)))
  (bind _spawnlocation (`local.SpawnLocation`))
  (bind (_bblockinghit _binitialoverlap _time _distance _location) (`GameplayStatics.BreakHitResult` (`PlayerController.GetHitResultUnderCursorByChannel` (`self.MaskPlayerController`) "TraceTypeQuery3" true)))
  (bind (_returnvalue_roll_2 _returnvalue_pitch_2 _returnvalue_yaw) (`KismetMathLibrary.BreakRotator` (`KismetMathLibrary.FindLookAtRotation` (`self.K2_GetActorLocation`) (`.Location` (`GameplayStatics.BreakHitResult` (`PlayerController.GetHitResultUnderCursorByChannel` (`self.MaskPlayerController`) "TraceTypeQuery3" true))))))
  ;[0 0 0 0.5 100] 里世界普攻
  ;;[0.15 0.15 0.15 0.5 36] 让玩家看向鼠标指针后攻击
  (`self.K2_SetActorRotation` (`KismetMathLibrary.MakeRotator` _returnvalue_roll _returnvalue_pitch _returnvalue_yaw))
  (switch `name` (`self.MaskID`)
    (:`0`
      ;;[0.15 0.15 0.15 0.5 36] 计算发射特效位置
      (set `local.SpawnLocation` (+ (+ _returnvalue_location (* (`self.GetActorForwardVector`) 50.0)) (0.0 0.0 30.0)) :!label _label)
      (set `local.SpawnRotation` _returnvalue_rotation)
      ;;[0.15 0 0.01129 0.5 36] 默认,钟馗(单发,近战)
      (bind _returnvalue (`|GetDataTableRow` "/Game/A_Mask/Data/DT_Mask.DT_Mask" (`self.MaskID`))
        (:`then`
          (`|SpawnActorFromClass` (`.BP_NormalAttack_46_482E8A0649AC3152C68F8A9F1A5E1B2C` (break `/Game/A_Mask/Data/S_Mask` _returnvalue)) (`KismetMathLibrary.MakeTransform` (`local.SpawnLocation`) (`local.SpawnRotation`)) "Undefined" "MultiplyWithRoot" null null))))
    (:`1`
      (goto _label))
    (:`2`
      ;;[0.15 0.15 0.15 0.5 36] 计算发射特效位置
      (set `local.SpawnLocation` (+ (+ _returnvalue_location_2 (* (`self.GetActorForwardVector`) 50.0)) (0.0 0.0 30.0)))
      (set `local.SpawnRotation` _returnvalue_rotation_2)
      ;;[0.1057 0.000112 0.15 0.5 36] 孟婆(扇形三发)
      (bind _returnvalue_2 (`|GetDataTableRow` "/Game/A_Mask/Data/DT_Mask.DT_Mask" (`self.MaskID`))
        (:`then`
          (`|ExecutionSequence`
            (:`then_0`
              (bind (_maskname _masktexture _attackvalue _uniquevalue _attacktexture _uniquetexturebackground _uniquetexturefill _maskmesh _bp_normalattack) (break `/Game/A_Mask/Data/S_Mask` _returnvalue_2))
              (`|SpawnActorFromClass` _bp_normalattack (`KismetMathLibrary.MakeTransform` _spawnlocation (`KismetMathLibrary.MakeRotator` _spawnrotation_roll _spawnrotation_pitch (- _spawnrotation_yaw 30.0))) "Undefined" "MultiplyWithRoot" null null))
            (:`then_1`
              (`|SpawnActorFromClass` _bp_normalattack (`KismetMathLibrary.MakeTransform` _spawnlocation (`local.SpawnRotation`)) "Undefined" "MultiplyWithRoot" null null))
            (:`then_2`
              (`|SpawnActorFromClass` _bp_normalattack (`KismetMathLibrary.MakeTransform` _spawnlocation (`KismetMathLibrary.MakeRotator` _spawnrotation_roll _spawnrotation_pitch (+ _spawnrotation_yaw 30.0))) "Undefined" "MultiplyWithRoot" null null))))))
    (:`3`
      ;;[0.15 0.15 0.15 0.5 36] 计算发射特效位置
      (if _bblockinghit
        (set `local.SpawnLocation` _location)
        (if (<= (`KismetMathLibrary.Vector_Distance` (`local.SpawnLocation`) (`self.K2_GetActorLocation`)) 1000.0)
          ;;[0.005619 0.1158 0.15 0.5 36] 无常(鼠标点闪电)
          (bind _returnvalue_3 (`|GetDataTableRow` "/Game/A_Mask/Data/DT_Mask.DT_Mask" (`self.MaskID`))
            (:`then`
              (`|SpawnActorFromClass` (`.BP_NormalAttack_46_482E8A0649AC3152C68F8A9F1A5E1B2C` (break `/Game/A_Mask/Data/S_Mask` _returnvalue_3)) (`KismetMathLibrary.MakeTransform` (`local.SpawnLocation`) (`local.SpawnRotation`)) "Undefined" "MultiplyWithRoot" null null)))
          (else
            ;; 超出射程
            (`NiagaraFunctionLibrary.SpawnSystemAtLocation` "/Game/Vefects/Easy_Shockwaves_VFX/VFX/Shockwaves/Particles/Color_Variation/VFX_Shockwave_01_Red_1s.VFX_Shockwave_01_Red_1s" (+ (`local.SpawnLocation`) (0.0 0.0 20.0)))))))))

(fn `StartMaskCD_MENGPO`
  (bind _wbp_overlay (`self.WBP_Overlay`))
  (bind _wbp_mask_mp (`/Game/A_Mask/Blueprint/UI/WBP_Overlay.WBP_Mask_MP` _wbp_overlay))
  ; Comment
  (`/Engine/EditorBlueprintResources/StandardMacros.IsValid` _wbp_overlay
    (:`Is Valid`
      (`/Engine/EditorBlueprintResources/StandardMacros.IsValid` _wbp_mask_mp
        (:`Is Valid`
          (`/Game/A_Mask/Blueprint/UI/SubWidget/WBP_Mask_MP.InitializeMaskCD` _wbp_mask_mp))))))

(fn `StartMaskCD_XBA`
  (bind _wbp_overlay (`self.WBP_Overlay`))
  (bind _wbp_mask_xba (`/Game/A_Mask/Blueprint/UI/WBP_Overlay.WBP_Mask_XBA` _wbp_overlay))
  ; Comment
  (`/Engine/EditorBlueprintResources/StandardMacros.IsValid` _wbp_overlay
    (:`Is Valid`
      (`/Engine/EditorBlueprintResources/StandardMacros.IsValid` _wbp_mask_xba
        (:`Is Valid`
          (`/Game/A_Mask/Blueprint/UI/SubWidget/WBP_Mask_XBA.InitializeMaskCD` _wbp_mask_xba))))))

(fn `StartMaskCD_ZHONGKUI`
  (bind _wbp_overlay (`self.WBP_Overlay`))
  (bind _wbp_mask_zk (`/Game/A_Mask/Blueprint/UI/WBP_Overlay.WBP_Mask_ZK` _wbp_overlay))
  ; Comment
  (`/Engine/EditorBlueprintResources/StandardMacros.IsValid` _wbp_overlay
    (:`Is Valid`
      (`/Engine/EditorBlueprintResources/StandardMacros.IsValid` _wbp_mask_zk
        (:`Is Valid`
          (`/Game/A_Mask/Blueprint/UI/SubWidget/WBP_Mask_ZK.InitializeMaskCD` _wbp_mask_zk))))))

(fn `StartMaskTime_MENGPO`
  (bind _wbp_overlay (`self.WBP_Overlay`))
  (bind _wbp_mask_mp (`/Game/A_Mask/Blueprint/UI/WBP_Overlay.WBP_Mask_MP` _wbp_overlay))
  ; Comment
  (`/Engine/EditorBlueprintResources/StandardMacros.IsValid` _wbp_overlay
    (:`Is Valid`
      (`/Engine/EditorBlueprintResources/StandardMacros.IsValid` _wbp_mask_mp
        (:`Is Valid`
          (`/Game/A_Mask/Blueprint/UI/SubWidget/WBP_Mask_MP.InitializeMaskTime` _wbp_mask_mp))))))

(fn `StartMaskTime_XBA`
  (bind _wbp_overlay (`self.WBP_Overlay`))
  (bind _wbp_mask_xba (`/Game/A_Mask/Blueprint/UI/WBP_Overlay.WBP_Mask_XBA` _wbp_overlay))
  ; Comment
  (`/Engine/EditorBlueprintResources/StandardMacros.IsValid` _wbp_overlay
    (:`Is Valid`
      (`/Engine/EditorBlueprintResources/StandardMacros.IsValid` _wbp_mask_xba
        (:`Is Valid`
          (`/Game/A_Mask/Blueprint/UI/SubWidget/WBP_Mask_XBA.InitializeMaskTime` _wbp_mask_xba))))))

(fn `StartMaskTime_ZHONGKUI`
  (bind _wbp_overlay (`self.WBP_Overlay`))
  (bind _wbp_mask_zk (`/Game/A_Mask/Blueprint/UI/WBP_Overlay.WBP_Mask_ZK` _wbp_overlay))
  ; Comment
  (`/Engine/EditorBlueprintResources/StandardMacros.IsValid` _wbp_overlay
    (:`Is Valid`
      (`/Engine/EditorBlueprintResources/StandardMacros.IsValid` _wbp_mask_zk
        (:`Is Valid`
          (`/Game/A_Mask/Blueprint/UI/SubWidget/WBP_Mask_ZK.InitializeMaskTime` _wbp_mask_zk))))))

(fn `SurfaceWorldSkill`
  (locals (SpawnRotation :type "Rotator Structure") (SpawnLocation :type "Vector Structure"))
  (bind (_returnvalue_location _returnvalue_rotation) (`KismetMathLibrary.BreakTransform` (`self.GetTransform`)))
  (bind (_returnvalue_roll _returnvalue_pitch) (`KismetMathLibrary.BreakRotator` (`self.K2_GetActorRotation`)))
  (bind (_bblockinghit _binitialoverlap _time _distance _location) (`GameplayStatics.BreakHitResult` (`PlayerController.GetHitResultUnderCursorByChannel` (`self.MaskPlayerController`) "TraceTypeQuery3" true)))
  (bind (_returnvalue_roll_2 _returnvalue_pitch_2 _returnvalue_yaw) (`KismetMathLibrary.BreakRotator` (`KismetMathLibrary.FindLookAtRotation` (`self.K2_GetActorLocation`) (`.Location` (`GameplayStatics.BreakHitResult` (`PlayerController.GetHitResultUnderCursorByChannel` (`self.MaskPlayerController`) "TraceTypeQuery3" true))))))
  ;[0.005722 0.15 0.01213 0.5 100] 表世界技能
  ;;[0.15 0.15 0.15 0.5 36] 让玩家看向鼠标指针后攻击
  (if (!= (`self.MaskID`) "0")
    (`self.K2_SetActorRotation` (`KismetMathLibrary.MakeRotator` _returnvalue_roll _returnvalue_pitch _returnvalue_yaw))
    (switch `name` (`self.MaskID`)
      (:`1`
        ;;[0.15 0.15 0.15 0.5 36] 计算发射特效位置
        (set `local.SpawnLocation` (+ _returnvalue_location (* (`self.GetActorForwardVector`) 50.0)))
        (set `local.SpawnRotation` _returnvalue_rotation)
        ;;[0.15 0 0.01129 0.5 36] 钟馗(碎墙)
        (bind _returnvalue (`|GetDataTableRow` "/Game/A_Mask/Data/DT_Mask.DT_Mask" (`self.MaskID`))
          (:`then`
            (`|SpawnActorFromClass` (`.BP_SurfaceWorldSkill_66_EC10F90F4DB8792CEF6B4BBCE91209A3` (break `/Game/A_Mask/Data/S_Mask` _returnvalue)) (`KismetMathLibrary.MakeTransform` (`local.SpawnLocation`) (`local.SpawnRotation`)) "Undefined" "MultiplyWithRoot" null null))))
      (:`2`
        ;;[0.15 0.15 0.15 0.5 36] 计算发射特效位置
        (set `local.SpawnLocation` (`SceneComponent.K2_GetComponentLocation` (`self.Mesh`)))
        ;;[0.1057 0.000112 0.15 0.5 36] 孟婆(灵视)
        (bind _returnvalue_2 (`|GetDataTableRow` "/Game/A_Mask/Data/DT_Mask.DT_Mask" (`self.MaskID`))))
      (:`3`
        ;;[0.15 0.15 0.15 0.5 36] 计算发射特效位置
        (if _bblockinghit
          (set `local.SpawnLocation` _location)
          (if (<= (`KismetMathLibrary.Vector_Distance` (`local.SpawnLocation`) (`self.K2_GetActorLocation`)) 1000.0)
            ;;[0.005619 0.1158 0.15 0.5 36] 谢必安(TP)
            (`self.K2_SetActorLocation` (+ (`local.SpawnLocation`) (0.0 0.0 50.0)) false true)
            (else
              ;; 超出射程
              (`NiagaraFunctionLibrary.SpawnSystemAtLocation` "/Game/Vefects/Easy_Shockwaves_VFX/VFX/Shockwaves/Particles/Color_Variation/VFX_Shockwave_01_Red_1s.VFX_Shockwave_01_Red_1s" (+ (`local.SpawnLocation`) (0.0 0.0 20.0))))))))))

(fn `TP`
  (bind _returnvalue (`NiagaraFunctionLibrary.SpawnSystemAtLocation` "/Game/A_Mask/VFX/Skill/NS_WorldTP.NS_WorldTP" (- (`SceneComponent.K2_GetComponentLocation` (`self.Mask`)) (0.0 0.0 130.0))))
  (`NiagaraComponent.SetVariableLinearColor` _returnvalue "Color" (`self.Player Color`)))

(fn `Ultimate`
  (locals (SpawnRotation :type "Rotator Structure") (SpawnLocation :type "Vector Structure"))
  ;[0 0.0117 0.15 0.5 100] 里世界大招
  (switch `name` (`self.MaskID`)
    (:`1`
      ;;[0.15 0.15 0.15 0.5 36] 计算发射特效位置
      (set `local.SpawnLocation` (+ (`SceneComponent.K2_GetComponentLocation` (`self.Mesh`)) (0.0 0.0 0.0)))
      (`self.Jump`)
      ;;[0.15 0 0.01129 0.5 36] 钟馗(地爆天星)
      (bind _returnvalue (`|GetDataTableRow` "/Game/A_Mask/Data/DT_Mask.DT_Mask" (`self.MaskID`))
        (:`then`
          (`|SpawnActorFromClass` (`.BP_UltimateAttack_60_BB479FCF49D6091A338216ADE009CD2B` (break `/Game/A_Mask/Data/S_Mask` _returnvalue)) (`KismetMathLibrary.MakeTransform` (`local.SpawnLocation`)) "Undefined" "MultiplyWithRoot" null null))))
    (:`2`
      ;;[0.15 0.15 0.15 0.5 36] 计算发射特效位置
      (set `local.SpawnLocation` (`SceneComponent.K2_GetComponentLocation` (`self.Mesh`)))
      ;;[0.1057 0.000112 0.15 0.5 36] 孟婆(彼岸花海)
      (bind _returnvalue_2 (`|GetDataTableRow` "/Game/A_Mask/Data/DT_Mask.DT_Mask" (`self.MaskID`))
        (:`then`
          (`|SpawnActorFromClass` (`.BP_UltimateAttack_60_BB479FCF49D6091A338216ADE009CD2B` (break `/Game/A_Mask/Data/S_Mask` _returnvalue_2)) (`KismetMathLibrary.MakeTransform` (`local.SpawnLocation`)) "Undefined" "MultiplyWithRoot" null null))))
    (:`3`
      ;;[0 0.09181 0.15 0.5 36] 谢必安(聚形散气)
      ;;;[0 0.15 0.01444 0.502] 无法被攻击
      (set `self.bCanBeAttack` false)
      ;;;[0 0.15 0.01444 0.502] 速度2x
      (set `CharacterMovementComponent.MaxWalkSpeed` (* (`self.CurrentSpeed`) 2.0) (`self.CharacterMovement`))
      (`KismetSystemLibrary.K2_SetTimer` null "Ultimate3End" 3.0))))

(fn `Ultimate3End`
  (locals (SpawnRotation :type "Rotator Structure") (SpawnLocation :type "Vector Structure"))
  (set `CharacterMovementComponent.MaxWalkSpeed` (`self.CurrentSpeed`) (`self.CharacterMovement`))
  (set `self.bCanBeAttack` true))

(fn `UserConstructionScript`
  (`parent.UserConstructionScript`))