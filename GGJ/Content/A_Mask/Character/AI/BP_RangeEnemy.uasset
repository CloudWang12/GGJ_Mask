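; BP_RangeEnemy is an AI enemy character whose ranged attack spawns a BP_LeftClick0 actor.
; The AIRangeAttack event prints a debug string, then spawns that actor at the location and rotation from CalculateSpawnTransform, with itself as owner and collision handling set to always spawn.
; BeginPlay, overlap, Tick and the construction script add no logic of their own.
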(event `/Game/A_Mask/Character/AI/BPI_AI.AI_RangeAttack`
  (bind (_rotation _location) (`self.CalculateSpawnTransform`))
  (`KismetSystemLibrary.PrintString` "RangeAttack")
  (`|SpawnActorFromClass` "/Game/A_Mask/Blueprint/Skill/BP_LeftClick0.BP_LeftClick0_C" (`KismetMathLibrary.MakeTransform` _location _rotation) "AlwaysSpawn" "MultiplyWithRoot" self null))

(fn `UserConstructionScript`
  (`parent.UserConstructionScript`))