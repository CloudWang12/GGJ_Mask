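; BP_NPC_Base is a base Blueprint for AI NPCs that provides health, damage handling and an enemy health bar.
; BeginPlay fills Health and caches the HealthBar widget as WBP_EnemyHealthBar.
; AnyDamage calls HealthChanged, which clamps Health and updates the bar's target percentage, then prints a debug message.
; Helpers report death at zero health and compute a spawn transform slightly ahead of and above the actor.
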(event `self.ReceiveBeginPlay`
  (bind _as_wbp_enemy_health_bar (`self.As WBP Enemy Health Bar`))
  (set `self.Health` (`self.MaxHealth`))
  (bind _aswbp_enemy_health_bar (cast `/Game/A_Mask/Blueprint/UI/SubWidget/WBP_EnemyHealthBar` (`WidgetComponent.GetUserWidgetObject` (`self.HealthBar`))))
  (set `self.As WBP Enemy Health Bar` _aswbp_enemy_health_bar)
  (`/Engine/EditorBlueprintResources/StandardMacros.IsValid` _as_wbp_enemy_health_bar
    (:`Is Valid`
      (set `/Game/A_Mask/Blueprint/UI/SubWidget/WBP_EnemyHealthBar.TargetPercentage` (/ (`self.Health`) (`self.MaxHealth`)) _as_wbp_enemy_health_bar))))

(event `self.ReceiveAnyDamage`
  (params (Damage :type "Float (single-precision)") (DamageType :type "DamageType Object Reference") (InstigatedBy :type "Controller Object Reference") (DamageCauser :type "Actor Object Reference"))
  (`self.HealthChanged` Damage)
  (`KismetSystemLibrary.PrintString` (`KismetStringLibrary.Concat_StrStr` "BP_NPC里的:" (`KismetSystemLibrary.GetDisplayName` self) "受到了" (`KismetStringLibrary.Conv_DoubleToString` Damage) "伤害,剩下" (`KismetStringLibrary.Conv_DoubleToString` (`self.Health`)) "滴血") true true (struct :`R` 1.0 :`G` 0.021687 :`A` 1.0)))

(fn `CalculateSpawnTransform`
  (returns (Rotation :type "Rotator Structure") (Location :type "Vector Structure"))
  (locals (SpawnRotation :type "Rotator Structure") (SpawnLocation :type "Vector Structure"))
  (bind (_returnvalue_location _returnvalue_rotation) (`KismetMathLibrary.BreakTransform` (`self.GetTransform`)))
  (bind _output_get (set `local.SpawnRotation` _returnvalue_rotation))
  (bind _output_get_2 (set `local.SpawnLocation` (+ (+ _returnvalue_location (* (`self.GetActorForwardVector`) 50.0)) (0.0 0.0 30.0))))
  (return _output_get _output_get_2))

(fn `HealthChanged`
  (params (HealthReleased :type "Float (double-precision)"))
  (bind _as_wbp_enemy_health_bar (`self.As WBP Enemy Health Bar`))
  (set `self.Health` (`KismetMathLibrary.FClamp` (- (`self.Health`) HealthReleased) 0.0 (`self.MaxHealth`)))
  (`/Engine/EditorBlueprintResources/StandardMacros.IsValid` _as_wbp_enemy_health_bar
    (:`Is Valid`
      (set `/Game/A_Mask/Blueprint/UI/SubWidget/WBP_EnemyHealthBar.TargetPercentage` (/ (`self.Health`) (`self.MaxHealth`)) _as_wbp_enemy_health_bar))))

(fn `IsDead`
  (returns (ReturnValue :type Boolean))
  (return (<= (`self.Health`) 0.0)))

(fn `UserConstructionScript`)