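; BP_RangeEnemy is a ranged AI enemy character that fires a spawnable actor at the player.
; The AIRangeAttack event plays a montage on the mesh and, on Notify Begin, spawns the configured class at the SpawnTransform component, rotated to look at player character 0.
; Timing the spawn to the montage notify keeps the shot in sync with the animation.
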(event `/Game/A_Mask/Character/AI/BPI_AI.AI_RangeAttack`
  (bind _returnvalue_location (`KismetMathLibrary.BreakTransform` (`SceneComponent.K2_GetComponentToWorld` (`self.SpawnTransform`))))
  (bind _notifyname (`|PlayMontage` (`self.Mesh`) (`self.Montage to Play`))
    (:`OnNotifyBegin`
      (switch `name` _notifyname
        (:`RangeAttack`
          (`|SpawnActorFromClass` (`self.SpawnableClass`) (`KismetMathLibrary.MakeTransform` _returnvalue_location (`KismetMathLibrary.FindLookAtRotation` _returnvalue_location (`self.K2_GetActorLocation` (`GameplayStatics.GetPlayerCharacter` 0)))) "AlwaysSpawn" "MultiplyWithRoot" null null))))))

(fn `UserConstructionScript`
  (`parent.UserConstructionScript`))