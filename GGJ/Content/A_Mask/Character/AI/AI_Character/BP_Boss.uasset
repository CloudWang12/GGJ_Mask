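; BP_Boss is the AI boss character, with a health bar widget, self-healing and a flying-sword attack.
; AnyDamage lowers clamped health and updates the bar, writing the pre-hit health ratio to the Blackboard only once health is at 30% or below.
; BOSSSelfHealing plays a defense montage while a looping timer restores health until completion.
; SwordAttack spawns a randomized volley of BP_FlySword actors targeting the player.
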(event `self.ReceiveBeginPlay`
  (`|ExecutionSequence`
    (:`then_0`
      (bind _returnvalue (`|CreateWidget` "/Game/A_Mask/Character/AI/AI_Character/WBP_BOSS.WBP_BOSS_C"))
      (bind _output_get (set `self.WBP_Boss_HealthBar` _returnvalue))
      (`UserWidget.AddToViewport` _output_get 0))))

(event `self.ReceiveAnyDamage`
  (params (Damage :type "Float (single-precision)") (DamageType :type "DamageType Object Reference") (InstigatedBy :type "Controller Object Reference") (DamageCauser :type "Actor Object Reference"))
  (if (`self.IsDead`)
    _
    (elif (`self.HealthLow30%`)
      (`self.CheckHealthPercentage` Damage)
      (else
        (`self.HealthDown` Damage)))))

(event `/Game/A_Mask/Character/AI/BPI_AI.BOSS_SelfHealing`
  (`|PlayMontage` (`self.Mesh`) "/Game/A_Mask/Asset/JR/Art/Characters/BOSS/Animation/SK_boss_Defense_Montage.SK_boss_Defense_Montage"
    (:`then`
      (bind _returnvalue (`KismetSystemLibrary.K2_SetTimerDelegate` (delegate `SelfHealing`) 1.0 true))
      (set `self.TH_SelfHealing` _returnvalue))
    (:`OnCompleted`
      (`KismetSystemLibrary.K2_ClearAndInvalidateTimerHandle` (`self.TH_SelfHealing`)))))

(event `SelfHealing`
  (`self.HealthUp` (`self.SelfHealingAccount`)))

(fn `CheckHealthPercentage`
  (params (HealthReleased :type "Float (double-precision)"))
  (`BlackboardComponent.SetValueAsFloat` (`AIBlueprintHelperLibrary.GetBlackboard` null) "Health" (/ (`self.Health`) (`self.MaxHealth`)))
  (`self.HealthDown` HealthReleased))

(fn `HealthDown`
  (params (HealthReleased :type "Float (double-precision)"))
  (bind _wbp_boss_healthbar (`self.WBP_Boss_HealthBar`))
  (set `self.Health` (`KismetMathLibrary.FClamp` (- (`self.Health`) HealthReleased) 0.0 (`self.MaxHealth`)))
  (`/Engine/EditorBlueprintResources/StandardMacros.IsValid` _wbp_boss_healthbar
    (:`Is Valid`
      (set `/Game/A_Mask/Character/AI/AI_Character/WBP_BOSS.TargetPercentage` (/ (`self.Health`) (`self.MaxHealth`)) _wbp_boss_healthbar))))

(fn `HealthLow30%`
  (returns (ReturnValue :type Boolean))
  (return (<= (/ (`self.Health`) (`self.MaxHealth`)) 0.3)))

(fn `HealthUp`
  (params (HealthIncrease :type "Float (double-precision)"))
  (bind _wbp_boss_healthbar (`self.WBP_Boss_HealthBar`))
  (set `self.Health` (`KismetMathLibrary.FClamp` (+ (`self.Health`) HealthIncrease) 0.0 (`self.MaxHealth`)))
  (`/Engine/EditorBlueprintResources/StandardMacros.IsValid` _wbp_boss_healthbar
    (:`Is Valid`
      (set `/Game/A_Mask/Character/AI/AI_Character/WBP_BOSS.TargetPercentage` (/ (`self.Health`) (`self.MaxHealth`)) _wbp_boss_healthbar))))

(fn `SwordAttack`
  (locals (Local_PlayerTarget :type "Actor Object Reference"))
  (bind _returnvalue (`KismetMathLibrary.RandomFloatInRange` -150.0 150.0))
  (bind _returnvalue_location (`KismetMathLibrary.BreakTransform` (`SceneComponent.K2_GetComponentToWorld` (`self.FlySwordLocation`))))
  (bind _returnvalue_2 (`GameplayStatics.GetActorOfClass` "/Game/A_Mask/Character/Player/BP_MaskPlayer.BP_MaskPlayer_C"))
  (bind _output_get (set `local.Local_PlayerTarget` _returnvalue_2))
  (for _ (range 14)
    (`|SpawnActorFromClass` "/Game/A_Mask/Blueprint/Skill/BOSS/BP_FlySword.BP_FlySword_C" (`KismetMathLibrary.MakeTransform` (+ _returnvalue_location (`KismetMathLibrary.MakeVector` _returnvalue _returnvalue _returnvalue)) (`KismetMathLibrary.MakeRotator` (.roll (`KismetMathLibrary.FindLookAtRotation` _returnvalue_location (`self.K2_GetActorLocation` (`local.Local_PlayerTarget`)))) (+ (.pitch (`KismetMathLibrary.FindLookAtRotation` _returnvalue_location (`self.K2_GetActorLocation` (`local.Local_PlayerTarget`)))) (`KismetMathLibrary.RandomFloatInRange` -90.0 90.0)) (+ (.yaw (`KismetMathLibrary.FindLookAtRotation` _returnvalue_location (`self.K2_GetActorLocation` (`local.Local_PlayerTarget`)))) 180.0 (`KismetMathLibrary.RandomFloatInRange` -60.0 60.0)))) "Undefined" "MultiplyWithRoot" null _output_get (`KismetMathLibrary.RandomFloatInRange` 4.0 6.0) (`KismetMathLibrary.RandomFloatInRange` 2000.0 4000.0) null)))

(fn `UserConstructionScript`)